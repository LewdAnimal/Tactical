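; BP_Grid is a grid actor that builds square or hexagon tiles as instanced static meshes in its Construction Script.
; SpawnGrid clears old instances, applies mesh and material from a shape data table, computes the bottom-left corner, then adds scaled instances.
; Hexagon grids step alternate rows per column for staggering.
; Sphere-trace ground snapping exists but is disconnected, and the tile location function ignores its index input.
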(event EventBeginPlay)

(event Collision|EventActorBeginOverlap
  (params (OtherActor :type Actor%20Object%20Reference)))

(event EventTick
  (params (DeltaSeconds :type Float%20%28single-precision%29)))

(fn ConstructionScript
  (CallFunction|SpawnGrid (Transformation|GetActorLocation) (Variables|Default|GetGridTileSize) (Variables|Default|GetGridTileCount) (Variables|Default|GetGridSape) false))

(fn SpawnGrid
  (params (CenterLocation :type Vector) (TileSize :type Vector) (TileCount :type Int%20Point%20Structure) (Sape :type E_GridShape%20Enum :default "NewEnumerator0") (UseEnviroment :type Boolean))
  (bind _returnvalue (CallFunction|GetCurrentShapeData))
  (bind _instancedstaticmesh (Variables|Default|GetInstancedStaticMesh))
  (bind (_meshsize _mesh _meshmaterial _flatmesh _flatbordermaterial) (Utilities|Struct|BreakS_GridShapeData _returnvalue))
  ;[0 0 0 1 14] [RU] Устанавливает значение переменых
  (Variables|Default|SetGridCenterLocation CenterLocation)
  (Variables|Default|SetGridTileSize TileSize)
  (Variables|Default|SetGridTileCount TileCount)
  (Variables|Default|SetGridSape Sape)
  (CallFunction|DestroyGrid)
  (Components|StaticMesh|SetStaticMesh _instancedstaticmesh _flatmesh)
  (Rendering|Material|SetMaterial _instancedstaticmesh 0 _flatbordermaterial)
  (CallFunction|SetGridOffsetfromGround (Variables|Default|GetGridOffsetFromGround))
  ;[0 0 0] Comment
  (bind (_center _bottomleft) (CallFunction|CalculateCenterandBotomLeft))
  (Variables|Default|SetGridCenterLocation _center)
  (Variables|Default|SetGridBottomLeftCornerLocation _bottomleft)
  (for _index (range 0 (- (.x (Variables|Default|GetGridTileCount)) 1))
    (LocalVariables|SetX _index)
    (if (Utilities|Enum|NotEqual(Enum) (Variables|Default|GetGridSape) "NewEnumerator2")
      (for _index_2 (range 0 (- (.y (Variables|Default|GetGridTileCount)) 1))
        (LocalVariables|SetY _index_2)
        (LocalVariables|SetIndex (Utilities|Struct|MakeIntPoint (LocalVariables|GetX) (LocalVariables|GetY)))
        (LocalVariables|SetTileTransform (Math|Transform|MakeTransform (+ (CallFunction|GetTitleLocationfromGridIndex (LocalVariables|GetIndex)) "0.000000,0.000000,2.000000") "0, 0, 0" (/ (Variables|Default|GetGridTileSize) (.MeshSize (Utilities|Struct|BreakS_GridShapeData (CallFunction|GetCurrentShapeData))))))
        ;[0 0 0] Comment
        (Components|InstancedStaticMesh|AddInstance (Variables|Default|GetInstancedStaticMesh) (LocalVariables|GetTileTransform) true))
      (else
        (for _index_3 (range (Math|Integer|SelectInt 0 1 (CallFunction|IsIntEven (LocalVariables|GetX))) (- (* (.y (Variables|Default|GetGridTileCount)) 2) 1))
          (LocalVariables|SetY _index_3)
          (Utilities|FlowControl|Sequence
            (:then_0
              (LocalVariables|SetIndex (Utilities|Struct|MakeIntPoint (LocalVariables|GetX) (LocalVariables|GetY)))
              (LocalVariables|SetTileTransform (Math|Transform|MakeTransform (+ (CallFunction|GetTitleLocationfromGridIndex (LocalVariables|GetIndex)) "0.000000,0.000000,2.000000") "0, 0, 0" (/ (Variables|Default|GetGridTileSize) (.MeshSize (Utilities|Struct|BreakS_GridShapeData (CallFunction|GetCurrentShapeData))))))
              (Components|InstancedStaticMesh|AddInstance (Variables|Default|GetInstancedStaticMesh) (LocalVariables|GetTileTransform) true))
            (:then_1
              (Math|Integer|IncrementInt _index_3))))))))

(fn GetCurrentShapeData
  (bind _gridsape (Variables|Default|GetGridSape))
  (bind _returnvalue (Utilities|String|EnumtoString _gridsape))
  (bind _returnvalue_2 (Utilities|GetDataTableRow "/Game/Blueprints/Core/Grid/GredShapes/DT_GridShapeData.DT_GridShapeData" (Utilities|String|StringToName _returnvalue))
    (:then
      (return _returnvalue_2))
    (:RowNotFound
      (Development|PrintString (Utilities|String|Append "Error - " _returnvalue) true true "(R=1.000000,G=0.000000,B=0.009181,A=1.000000)" 5.0))))

(fn DestroyGrid
  (Components|InstancedStaticMesh|ClearInstances (Variables|Default|GetInstancedStaticMesh)))

(fn CalculateCenterandBotomLeft
  (bind _gridtilecount (Variables|Default|GetGridTileCount))
  (bind _gridtilecount_2 (Variables|Default|GetGridTileCount))
  (bind _iseven (CallFunction|IsIntEven (.y _gridtilecount_2)))
  (bind _iseven_2 (CallFunction|IsIntEven (.x _gridtilecount_2)))
  (bind _returnvalue (Math|Float|SelectFloat 0.0 1.0 _iseven_2))
  (bind _returnvalue_2 (Math|Float|SelectFloat 0.0 1.0 _iseven))
  (bind _returnvalue_3 (- _gridtilecount (Math|Vector2D|MakeVector2D _returnvalue _returnvalue_2)))
  (switch Utilities|FlowControl|Switch|SwitchonE_GridShape (Variables|Default|GetGridSape)
    (:NewEnumerator1
      (LocalVariables|SetC (CallFunction|SnapVectortoVector (Variables|Default|GetGridCenterLocation) (Variables|Default|GetGridTileSize)))
      (return (Variables|Default|GetGridCenterLocation) (- (Variables|Default|GetGridCenterLocation) (* (/ (Math|Vector2D|MakeVector2D (.x _returnvalue_3) (.y _returnvalue_3)) (Math|Vector2D|MakeVector2D 2.0 2.0)) (Math|Conversions|ToVector2D(Vector) (Variables|Default|GetGridTileSize))))))
    (:NewEnumerator2
      (LocalVariables|SetC (CallFunction|SnapVectortoVector (Variables|Default|GetGridCenterLocation) (* (Variables|Default|GetGridTileSize) "1.500000,1.000000,1.000000")))
      (return (Variables|Default|GetGridCenterLocation) (- (Variables|Default|GetGridCenterLocation) (CallFunction|SnapVectortoVector (* (/ (Variables|Default|GetGridTileCount) "(X=3.000000,Y=2.000000)") (Math|Conversions|ToVector2D(Vector) (Variables|Default|GetGridTileSize))) (* (Variables|Default|GetGridTileSize) "1.500000,1.000000,1.000000")))))))

(fn GetTitleLocationfromGridIndex
  (params (InputPin :type Int%20Point%20Structure))
  (return (+ (Variables|Default|GetGridBottomLeftCornerLocation) (* (Variables|Default|GetGridTileSize) (* "" (Utilities|Select :Index (Variables|Default|GetGridSape) :NewEnumerator0 "0.000000,0.000000,1.000000" :NewEnumerator1 "1.000000,1.000000,1.000000" :NewEnumerator2 "0.750000,0.500000,1.000000"))))))

(fn TracerforGround
  (params (Location :type Vector))
  (Variables|Default|SetRadius (/ (.x (Variables|Default|GetGridTileSize)) 3.0))
  (bind _outhits (Collision|MultiSphereTraceByChannel (+ Location "0.000000,0.000000,1000.000000") (- Location "0.000000,0.000000,1000.000000") (Variables|Default|GetRadius) "TraceTypeQuery3" false 0 "ForDuration"))
  (if (> (Utilities|Array|Length _outhits) 0)
    (return (Math|Vector|MakeVector (.x Location) (.y Location) (Math|Float|SnapToGrid(Float) (- (.Z (Math|Vector|BreakVector (.Location (Collision|BreakHitResult (Utilities|Array|Get(acopy) _outhits))))) (Variables|Default|GetRadius)) (.z (Variables|Default|GetGridTileSize)))) true)
    (else
      (return Location false))))

(fn SetGridOffsetfromGround
  (params (Offset :type Float%20%28double-precision%29))
  (Variables|Default|SetGridOffsetFromGround Offset)
  (Transformation|SetWorldLocation (Variables|Default|GetInstancedStaticMesh) (Math|Vector|MakeVector 0.0 0.0 (Variables|Default|GetGridOffsetFromGround)) false false))